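; A reusable box trigger actor that calls its AwesomeTriggerActivated event dispatcher when a suitably tagged actor begins overlapping it.
; Overlaps count only while the trigger is enabled and the actor carries one of the configured tags.
; An optional DoOnce gate limits activation to once until reset, and events toggle the enabled state.
; The construction script applies the configurable box extent and label text.
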(event OnComponentBeginOverlap(Trigger)
  (params (OverlappedComponent :type Primitive%20Component%20Object%20Reference) (OtherActor :type Actor%20Object%20Reference) (OtherComp :type Primitive%20Component%20Object%20Reference) (OtherBodyIndex :type Integer) (bFromSweep :type Boolean) (SweepResult :type Hit%20Result%20Structure%20%28by%20ref%29))
  (Variables|Default|SetActorHasCorrectTag false)
  (for _array_element (Variables|Default|GetActorHasTagToActivate)
    (if (Actor|ActorHasTag OtherActor _array_element)
      (if (Variables|Default|GetEnable)
        (Variables|Default|SetActorHasCorrectTag true))))
  (if (Variables|Default|GetActorHasCorrectTag)
    (if (Variables|Default|GetDoOnce)
      (Utilities|FlowControl|DoOnce false
        (:Completed
          _)))
    (Default|CallAwesomeTriggerActivatedDisplatcher)))

(event Custom|EnableTrigger
  (Variables|Default|SetEnable true))

(event Custom|DisableTrigger
  (Variables|Default|SetEnable false))

(event Custom|ResetDoOnce
  (Utilities|FlowControl|DoOnce false) ; enters at Reset
)

(fn ConstructionScript
  (Components|Box|SetBoxExtent (Variables|Default|GetTrigger) (Variables|Default|GetTriggerExtent) true)
  (Rendering|Components|TextRender|SetText (Variables|Default|GetMyTrigger) (Variables|Default|GetTriggerText)))