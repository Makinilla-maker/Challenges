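; Child-actor example of a complex look-at interaction that glows, shows HUD prompts and notifies its parent actor when used.
; ConstructionFuntion sizes both triggers from InteractStructure and collects parent meshes by name substring for stencil-colored outlines.
; Player overlap with the box toggles custom depth on those meshes.
; Interacting calls ComplexInteractMessage on the parent, optionally only once, disabling the glow and look-at sphere until re-enabled.
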(event OnComponentBeginOverlap(Box)
  (params (OverlappedComponent :type Primitive%20Component%20Object%20Reference) (OtherActor :type Actor%20Object%20Reference) (OtherComp :type Primitive%20Component%20Object%20Reference) (OtherBodyIndex :type Integer) (bFromSweep :type Boolean) (SweepResult :type Hit%20Result%20Structure%20%28by%20ref%29))
  (if (.InteractionEnable (Utilities|Struct|BreakComplexLookAtStructure (Variables|Default|GetInteractStructure)))
    (if (Actor|ActorHasTag OtherActor "Player")
      (CallFunction|BeginGlow))))

(event OnComponentEndOverlap(Box)
  (params (OverlappedComponent :type Primitive%20Component%20Object%20Reference) (OtherActor :type Actor%20Object%20Reference) (OtherComp :type Primitive%20Component%20Object%20Reference) (OtherBodyIndex :type Integer))
  (if (.InteractionEnable (Utilities|Struct|BreakComplexLookAtStructure (Variables|Default|GetInteractStructure)))
    (if (Actor|ActorHasTag OtherActor "Player")
      (CallFunction|EndGlow))))

(event Custom|ResetDoOnce
  (Utilities|FlowControl|DoOnce false) ; enters at Reset
)

(event Custom|ShowInteractMessage
  (bind _returnvalue (Game|GetPlayerCharacter 0))
  (bind _interactstructure (Variables|Default|GetInteractStructure))
  (bind (_interactionenable _doonce _glowoutlinetriggerextents _lookattriggerradious _glowparentcomponents _glowingcolor _interacttext _interactiontodotext _holdtointeract _audio) (Utilities|Struct|BreakComplexLookAtStructure _interactstructure))
  (bind _asbp_first_person_character (Utilities|Casting|CastToBP_FirstPersonCharacter _returnvalue))
  (bind _interacthud (Variables|/Game/Corridor/Blueprints/BP_FirstPersonCharacter.BP_FirstPersonCharacter_C|GetInteractHUD _asbp_first_person_character))
  (Utilities|FlowControl|DoOnce false
    (:Completed
      (if _interactionenable
        (Default|ShowHUDMessage _interacthud (Utilities|Text|ToText(String) (Utilities|String|Append _interacttext " | " _interactiontodotext)) _audio)
        (else
          (Default|HideHUD _interacthud))))))

(event Custom|ResetDoOnceHUD
  (bind _returnvalue (Game|GetPlayerCharacter 0))
  (bind _interactstructure (Variables|Default|GetInteractStructure))
  (bind (_interactionenable _doonce _glowoutlinetriggerextents _lookattriggerradious _glowparentcomponents _glowingcolor _interacttext _interactiontodotext _holdtointeract _audio) (Utilities|Struct|BreakComplexLookAtStructure _interactstructure))
  (bind _asbp_first_person_character (Utilities|Casting|CastToBP_FirstPersonCharacter _returnvalue))
  (bind _interacthud (Variables|/Game/Corridor/Blueprints/BP_FirstPersonCharacter.BP_FirstPersonCharacter_C|GetInteractHUD _asbp_first_person_character))
  (Utilities|FlowControl|DoOnce false) ; enters at Reset
)

(event Custom|EndGlow
  (for _array_element (Variables|Default|GetGlowingStaticMeshComponents)
    (Rendering|SetRenderCustomDepth _array_element false)))

(event Custom|BeginGlow
  (for _array_element (Variables|Default|GetGlowingStaticMeshComponents)
    (Rendering|SetRenderCustomDepth _array_element true)))

(event Custom|EnableInteract
  (Collision|SetCollisionEnabled (Variables|Default|GetSphere) "QueryAndPhysics")
  (Utilities|Struct|SetmembersinComplexLookAtStructure (Variables|Default|GetInteractStructure) true))

(event Collision|EventActorBeginOverlap
  (params (OtherActor :type Actor%20Object%20Reference)))

(event EventTick
  (params (DeltaSeconds :type Float%20%28single-precision%29)))

(event EventComplexInteract
  (bind _interactstructure (Variables|Default|GetInteractStructure))
  (bind (_interactionenable _doonce) (Utilities|Struct|BreakComplexLookAtStructure _interactstructure))
  (if _interactionenable
    (if _doonce
      (Utilities|FlowControl|DoOnce false
        (:Completed
          (CallFunction|EndGlow)
          (Collision|SetCollisionEnabled (Variables|Default|GetSphere) "NoCollision")
          (Utilities|Struct|SetmembersinComplexLookAtStructure (Variables|Default|GetInteractStructure) false))))
    (Class|ComplexInteractionInterface|ComplexInteract(Message) (Actor|GetParentActor))))

(fn ConstructionScript)

(fn ConstructionFuntion
  (bind _interactstructure (Variables|Default|GetInteractStructure))
  (bind (_interactionenable _doonce _glowoutlinetriggerextents _lookattriggerradious) (Utilities|Struct|BreakComplexLookAtStructure _interactstructure))
  (Components|Box|SetBoxExtent (Variables|Default|GetBox) _glowoutlinetriggerextents true)
  (Components|Sphere|SetSphereRadius (Variables|Default|GetSphere) _lookattriggerradious true)
  (for _array_element (Actor|GetComponentsByClass (Actor|GetParentActor) "/Script/Engine.StaticMeshComponent")
    (for _array_element_2 (.GlowParentCOmponents (Utilities|Struct|BreakComplexLookAtStructure (Variables|Default|GetInteractStructure)))
      (if (Utilities|String|Contains (Utilities|GetObjectName _array_element) _array_element_2)
        (Utilities|Array|Add (Variables|Default|GetGlowingStaticMeshComponents) _array_element))))
  (for _array_element_3 (Variables|Default|GetGlowingStaticMeshComponents)
    (Rendering|SetCustomDepthStencilValue _array_element_3 (+ (.GlowingColor (Utilities|Struct|BreakComplexLookAtStructure (Variables|Default|GetInteractStructure))) 1))))