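; Sliding door that opens when an actor tagged Player enters its trigger box and closes when they leave.
; BeginPlay converts the DoorDirection enum into a movement offset, which a timeline lerps the mesh's relative location toward, reversing on exit.
; Both overlaps fire open/close dispatchers, even for Broken doors, which stay still and play an invalid-action sound at world origin on entry.
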(event OnComponentBeginOverlap(Box)
  (params (OverlappedComponent :type Primitive%20Component%20Object%20Reference) (OtherActor :type Actor%20Object%20Reference) (OtherComp :type Primitive%20Component%20Object%20Reference) (OtherBodyIndex :type Integer) (bFromSweep :type Boolean) (SweepResult :type Hit%20Result%20Structure%20%28by%20ref%29))
  (if (Actor|ActorHasTag OtherActor "Player")
    (Default|CallStartDoorOpenDispatcher)
    (Development|PrintString (Utilities|String|EnumtoString (Variables|Default|GetDoorDirection)))
    (if (Utilities|Enum|Equal(Enum) (Variables|Default|GetDoorDirection) "NewEnumerator4")
      (Audio|PlaySoundatLocation "/Engine/VREditor/Sounds/UI/Invalid_Action.Invalid_Action" "0, 0, 0" "0, 0, 0" 1.0 1.0 0.0 0 0 0 0)
      (else
        (Audio|PlaySoundatLocation "/Engine/VREditor/Sounds/UI/Floating_UI_Close.Floating_UI_Close" (Transformation|GetWorldLocation (Variables|Default|GetSlidingDoor)) "0, 0, 0" 0.5 1.0 0.0 0 0 0 0)
        (bind _alphatrack (Timeline|SlidingDoor%20Timeline Play)
          (:Update
            (Transformation|SetRelativeLocation (Variables|Default|GetSlidingDoor) (Math|Vector|Lerp(Vector) "0, 0, 0" (Variables|Default|GetdirectionMovement) _alphatrack) false false)))))))

(event OnComponentEndOverlap(Box)
  (params (OverlappedComponent :type Primitive%20Component%20Object%20Reference) (OtherActor :type Actor%20Object%20Reference) (OtherComp :type Primitive%20Component%20Object%20Reference) (OtherBodyIndex :type Integer))
  (if (Actor|ActorHasTag OtherActor "Player")
    (Default|CallStartDoorCloseDispatcher)
    (if (not (Utilities|Enum|Equal(Enum) (Variables|Default|GetDoorDirection) "NewEnumerator4"))
      (Audio|PlaySoundatLocation "/Engine/VREditor/Sounds/UI/Dockable_Window_Close.Dockable_Window_Close" (Transformation|GetWorldLocation (Variables|Default|GetSlidingDoor)) "0, 0, 0" 0.5 1.0 0.0 0 0 0 0)
      (bind _alphatrack (Timeline|SlidingDoor%20Timeline Reverse)
        (:Update
          (Transformation|SetRelativeLocation (Variables|Default|GetSlidingDoor) (Math|Vector|Lerp(Vector) "0, 0, 0" (Variables|Default|GetdirectionMovement) _alphatrack) false false))))))

(event EventBeginPlay
  (CallFunction|SetDoorType (Variables|Default|GetDoorDirection)))

(fn ConstructionScript)

(fn SetDoorType
  (params (NewParam :type DoorDir%20Enum :default "NewEnumerator0"))
  (switch Utilities|FlowControl|Switch|SwitchonDoorDir NewParam
    (:NewEnumerator0
      (Variables|Default|SetdirectionMovement "0.000000,0.000000,350.000000")
      (Variables|Default|SetDoorDirection "NewEnumerator0"))
    (:NewEnumerator1
      (Variables|Default|SetdirectionMovement "0.000000,0.000000,-360.000000")
      (Variables|Default|SetDoorDirection "NewEnumerator1"))
    (:NewEnumerator2
      (Variables|Default|SetdirectionMovement "180.000000,0.000000,0.000000")
      (Variables|Default|SetDoorDirection "NewEnumerator2"))
    (:NewEnumerator3
      (Variables|Default|SetdirectionMovement "-180.000000,0.000000,0.000000")
      (Variables|Default|SetDoorDirection "NewEnumerator3"))
    (:NewEnumerator4
      (Variables|Default|SetdirectionMovement "0.000000,0.000000,100.000000")
      (Variables|Default|SetDoorDirection "NewEnumerator4"))))