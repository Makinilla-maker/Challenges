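; Trigger volume actor that fires a look-at dispatcher when the player camera looks at a linked probe actor.
; While enabled, overlaps by actors with an activating tag switch Tick on at entry and off at exit.
; Tick line-traces along the camera's forward vector and fires on hitting the probe, optionally only once until reset.
; The construction script applies box extent, label text and probe sphere radius.
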(event OnComponentBeginOverlap(Trigger)
  (params (OverlappedComponent :type Primitive%20Component%20Object%20Reference) (OtherActor :type Actor%20Object%20Reference) (OtherComp :type Primitive%20Component%20Object%20Reference) (OtherBodyIndex :type Integer) (bFromSweep :type Boolean) (SweepResult :type Hit%20Result%20Structure%20%28by%20ref%29))
  (Variables|Default|SetActorHasCorrectTag false)
  (for _array_element (Variables|Default|GetActorHasTagToActivate)
    (if (Actor|ActorHasTag OtherActor _array_element)
      (if (Variables|Default|GetEnable)
        (Variables|Default|SetActorHasCorrectTag true)
        (Actor|Tick|SetActorTickEnabled true))))
  (if (Variables|Default|GetActorHasCorrectTag)
    _))

(event OnComponentEndOverlap(Trigger)
  (params (OverlappedComponent :type Primitive%20Component%20Object%20Reference) (OtherActor :type Actor%20Object%20Reference) (OtherComp :type Primitive%20Component%20Object%20Reference) (OtherBodyIndex :type Integer))
  (Variables|Default|SetActorHasCorrectTag false)
  (for _array_element (Variables|Default|GetActorHasTagToActivate)
    (if (Actor|ActorHasTag OtherActor _array_element)
      (if (Variables|Default|GetEnable)
        (Variables|Default|SetActorHasCorrectTag true)
        (Actor|Tick|SetActorTickEnabled false))))
  (if (Variables|Default|GetActorHasCorrectTag)
    _))

(event Custom|EnableLookAtTrigger
  (Variables|Default|SetEnable true))

(event Custom|DisableLookAtTrigger
  (Variables|Default|SetEnable false))

(event Custom|ResetDoOnce
  (Utilities|FlowControl|DoOnce false) ; enters at Reset
)

(event EventTick
  (params (DeltaSeconds :type Float%20%28single-precision%29))
  (bind _returnvalue (Game|GetPlayerCameraManager 0))
  (bind _returnvalue_2 (Camera|GetCameraLocation _returnvalue))
  (bind (_outhit _returnvalue_3) (Collision|LineTraceByChannel _returnvalue_2 (+ _returnvalue_2 (* (Transformation|GetActorForwardVector _returnvalue) "50000.000000,50000.000000,50000.000000")) "TraceTypeQuery2" false 0 "None"))
  (if _returnvalue_3
    (if (== (.HitActor (Collision|BreakHitResult _outhit)) (Variables|Default|GetLookAtProveActor))
      (if (Variables|Default|GetDoOnce)
        (Utilities|FlowControl|DoOnce false
          (:Completed
            _)))
      (Default|CallLookatDispatcher))))

(fn ConstructionScript
  (Components|Box|SetBoxExtent (Variables|Default|GetTrigger) (Variables|Default|GetTriggerExtent) true)
  (Rendering|Components|TextRender|SetText (Variables|Default|GetMyTrigger) (Variables|Default|GetTriggerText))
  (Components|Sphere|SetSphereRadius (Variables|/Game/Corridor/Blueprints/LookAt/LookAtTrigger.LookAtTrigger_C|GetSphere (Variables|Default|GetLookAtProveActor)) (Variables|Default|GetProbeSize) true))